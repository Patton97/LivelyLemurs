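; BP_door_big is a big double door with a two-piece lock that animates when its trigger volume is overlapped.
; Timelines chain through Finished: the lock rotates, its pieces separate, then the door halves slide apart carrying them.
; Opening completion sets VarOpen and immediately runs the closing sequence in reverse order, though VarOpen is never reset to false.
; Motion offsets initial transforms cached at BeginPlay, recapturing lock locations between stages.
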(event OnComponentBeginOverlap(trigger)
  (params (OverlappedComponent :type Primitive%20Component%20Object%20Reference) (OtherActor :type Actor%20Object%20Reference) (OtherComp :type Primitive%20Component%20Object%20Reference) (OtherBodyIndex :type Integer) (bFromSweep :type Boolean) (SweepResult :type Hit%20Result%20Structure%20%28by%20ref%29))
  ;[1 1 1] When player enters trigger volume, begin animation
  (CallFunction|Animate))

(event Custom|Animation%20door_move
  ;[1 1 1] Animate the movement of the doors
  (if (Variables|Default|Getvar_open)
    (bind _door_loc (Timeline|door_open ReverseFromEnd)
      (:Update
        (Transformation|SetRelativeLocation (Variables|Default|Getdoor_left) (- (Variables|Default|Getdoor_left_init_loc) _door_loc) false false)
        (Transformation|SetRelativeLocation (Variables|Default|Getlock_bottom) (- (Variables|Default|Getlock_bottom_init_loc) _door_loc) false false)
        (Transformation|SetRelativeLocation (Variables|Default|Getdoor_right) (+ (Variables|Default|Getdoor_right_init_loc) _door_loc) false false)
        (Transformation|SetRelativeLocation (Variables|Default|Getlock_top) (+ (Variables|Default|Getlock_top_init_loc) _door_loc) false false))
      (:Finished
        (if (Variables|Default|Getvar_open)
          ;;[1 1 1] Recapture location of lock_top and lock_bottom after lock_open
          (Variables|Default|Setlock_top_init_loc (Variables|/Script/Engine.SceneComponent|GetRelativeLocation (Variables|Default|Getlock_top)))
          (Variables|Default|Setlock_bottom_init_loc (Variables|/Script/Engine.SceneComponent|GetRelativeLocation (Variables|Default|Getlock_bottom)))
          (CallFunction|AnimationLockMove)
          (else
            (Variables|Default|Setvar_open true)
            (CallFunction|Animate)))))
    (else
      (Timeline|door_open PlayFromStart))))

(event Custom|animate
  ;[1 1 1] When animation begins, check if door is already open
  (if (Variables|Default|Getvar_open)
    (CallFunction|AnimationDoorMove)
    (else
      (CallFunction|AnimationLockRotate))))

(event Custom|Animation%20lock_rotate
  (bind _lock_top_init_rot (Variables|Default|Getlock_top_init_rot))
  (bind _lock_bottom_init_rot (Variables|Default|Getlock_bottom_init_rot))
  (bind (_roll _pitch _yaw) (Math|Rotator|BreakRotator _lock_top_init_rot))
  (bind (_roll_2 _pitch_2 _yaw_2) (Math|Rotator|BreakRotator _lock_bottom_init_rot))
  ;[1 1 1] Animate the rotation of the lock
  (if (Variables|Default|Getvar_open)
    (bind _rot_angle (Timeline|lock_rotate ReverseFromEnd)
      (:Update
        (Transformation|SetRelativeRotation (Variables|Default|Getlock_top) (Math|Rotator|MakeRotator (+ _rot_angle _roll) _pitch _yaw) false false)
        (Transformation|SetRelativeRotation (Variables|Default|Getlock_bottom) (Math|Rotator|MakeRotator (- _rot_angle _roll_2) _pitch_2 _yaw_2) false false))
      (:Finished
        (if (Variables|Default|Getvar_open)
          (Variables|Default|Setvar_open true)
          (else
            (CallFunction|AnimationLockMove)))))
    (else
      (Timeline|lock_rotate PlayFromStart))))

(event Custom|Animation%20lock_move
  ;[1 1 1] Animate the movement of the separate lock pieces
  (if (Variables|Default|Getvar_open)
    (bind _lock_loc (Timeline|lock_close PlayFromStart)
      (:Update
        (Transformation|SetRelativeLocation (Variables|Default|Getlock_top) (+ (Variables|Default|Getlock_top_init_loc) _lock_loc) false false)
        (Transformation|SetRelativeLocation (Variables|Default|Getlock_bottom) (- (Variables|Default|Getlock_bottom_init_loc) _lock_loc) false false))
      (:Finished
        (CallFunction|AnimationLockRotate)))
    (else
      (bind _lock_loc_2 (Timeline|lock_open PlayFromStart)
        (:Update
          (Transformation|SetRelativeLocation (Variables|Default|Getlock_top) (- (Variables|Default|Getlock_top_init_loc) _lock_loc_2) false false)
          (Transformation|SetRelativeLocation (Variables|Default|Getlock_bottom) (+ (Variables|Default|Getlock_bottom_init_loc) _lock_loc_2) false false))
        (:Finished
          ;;[1 1 1] Recapture location of lock_top and lock_bottom after lock_open
          (Variables|Default|Setlock_top_init_loc (Variables|/Script/Engine.SceneComponent|GetRelativeLocation (Variables|Default|Getlock_top)))
          (Variables|Default|Setlock_bottom_init_loc (Variables|/Script/Engine.SceneComponent|GetRelativeLocation (Variables|Default|Getlock_bottom)))
          (CallFunction|AnimationDoorMove))))))

(event EventBeginPlay
  (bind _lock_bottom (Variables|Default|Getlock_bottom))
  (bind _lock_top (Variables|Default|Getlock_top))
  ;[1 1 1] Capture initial location vector and rotation angle of components
  (Variables|Default|Setlock_top_init_rot (Variables|/Script/Engine.SceneComponent|GetRelativeRotation _lock_top))
  (Variables|Default|Setlock_top_init_loc (Variables|/Script/Engine.SceneComponent|GetRelativeLocation _lock_top))
  (Variables|Default|Setlock_bottom_init_rot (Variables|/Script/Engine.SceneComponent|GetRelativeRotation _lock_bottom))
  (Variables|Default|Setlock_bottom_init_loc (Variables|/Script/Engine.SceneComponent|GetRelativeLocation _lock_bottom))
  (Variables|Default|Setdoor_left_init_loc (Variables|/Script/Engine.SceneComponent|GetRelativeLocation (Variables|Default|Getdoor_left)))
  (Variables|Default|Setdoor_right_init_loc (Variables|/Script/Engine.SceneComponent|GetRelativeLocation (Variables|Default|Getdoor_right))))

(fn ConstructionScript)